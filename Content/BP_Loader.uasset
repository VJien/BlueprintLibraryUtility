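; Actor that loads mesh files from disk at runtime and builds them as procedural meshes.
; Init passes a path list to LoadMeshesWithDelay, which loads one file at a time with a delay between, creating a component per section and stopping on a failed load.
; Refresh rebuilds a single mesh and sets material colors, opacity and diffuse texture, but its construction-script call and all dynamic material creation are disconnected.
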(event `self.ReceiveBeginPlay`)

(event `Init`
  (params (Pathes :type "Array of String"))
  (`self.LoadMeshesWithDelay` Pathes 2.0))

(fn `Refresh`
  (bind (_isvalid _width _height _returnvalue) (`Flib_IO.LoadTexture2DFromFile` (`KismetStringLibrary.Concat_StrStr` (`BlueprintPathsLibrary.ProjectPluginsDir`) "BlueprintLibraryUtility/Content/" (`self.T_Dif_RelateivePath`))))
  (bind _returnvalue_2 (`Flib_IO.LoadMeshData` (`self.MeshRelativePath`) (`self.Config`)))
  (bind (_bsuccess _meshnumbers _meshdata) (break `LoadedMeshData` _returnvalue_2))
  (if _bsuccess
    (`|ExecutionSequence`
      (:`then_0`
        (for (_array_element _array_index) _meshdata
          (bind (_vertices _triangles _normals _uv0 _vertexcolors _tangents) (break `MeshData` _array_element))
          (`ProceduralMeshComponent.CreateMeshSection_LinearColor` :`self` (`self.ProceduralMesh`) :`SectionIndex` _array_index :`Vertices` _vertices :`Triangles` _triangles :`Normals` _normals :`UV0` _uv0 :`VertexColors` _vertexcolors :`Tangents` _tangents)))
      (:`then_1`
        (bind _returnvalue_3 (`|GetMatProperty` (`self.GetMeshFilePath`) "COLOR_DIFFUSE"))
        (`MaterialInstanceDynamic.SetVectorParameterValue` (`self.Mat`) "Dif" _returnvalue_3))
      (:`then_2`
        (bind _returnvalue_4 (`|GetMatProperty` (`self.GetMeshFilePath`) "COLOR_EMISSIVE"))
        (`MaterialInstanceDynamic.SetVectorParameterValue` (`self.Mat`) "Em" _returnvalue_4))
      (:`then_3`
        (bind _returnvalue_5 (`|GetMatProperty` (`self.GetMeshFilePath`) "OPACITY"))
        (`MaterialInstanceDynamic.SetScalarParameterValue` (`self.Mat`) "Op" _returnvalue_5))
      (:`then_4`
        (if _isvalid
          (`MaterialInstanceDynamic.SetTextureParameterValue` (`self.Mat`) "T_Dif" _returnvalue))))))

(fn `UserConstructionScript`)