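; Actor Blueprint that loads a mesh file into a procedural mesh at construction, using a path relative to BlueprintLibraryUtility plugin content.
; The construction script calls LoadMeshData, then creates one mesh section and M_MeshLoader dynamic material per returned entry.
; It then applies the file's index-0 diffuse, emissive and opacity properties to the stored material, which is only the last one created.
; The event graph has no runtime logic.
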(event `self.ReceiveBeginPlay`)

(fn `UserConstructionScript`
  (bind _proceduralmesh (`self.ProceduralMesh`))
  (bind _returnvalue (`Flib_IO.LoadMeshData` (`self.GetFilePath`) (`self.Config`)))
  (bind (_bsuccess _meshnumbers _meshdata) (break `LoadedMeshData` _returnvalue))
  (if _bsuccess
    (`|ExecutionSequence`
      (:`then_0`
        (for (_array_element _array_index) _meshdata
          (bind (_vertices _triangles _normals _uv0 _vertexcolors _tangents) (break `MeshData` _array_element))
          (`ProceduralMeshComponent.CreateMeshSection_LinearColor` :`self` _proceduralmesh :`SectionIndex` _array_index :`Vertices` _vertices :`Triangles` _triangles :`Normals` _normals :`UV0` _uv0 :`VertexColors` _vertexcolors :`Tangents` _tangents)
          (bind _returnvalue_2 (`KismetMaterialLibrary.CreateDynamicMaterialInstance` "/BlueprintLibraryUtility/M_MeshLoader.M_MeshLoader"))
          (bind _output_get (set `self.Mat` _returnvalue_2))
          (`PrimitiveComponent.SetMaterial` _proceduralmesh _array_index _output_get)))
      (:`then_1`
        (bind _returnvalue_3 (`|GetMatProperty` (`self.GetFilePath`) "COLOR_DIFFUSE"))
        (`MaterialInstanceDynamic.SetVectorParameterValue` (`self.Mat`) "Dif" _returnvalue_3))
      (:`then_2`
        (bind _returnvalue_4 (`|GetMatProperty` (`self.GetFilePath`) "COLOR_EMISSIVE"))
        (`MaterialInstanceDynamic.SetVectorParameterValue` (`self.Mat`) "Em" _returnvalue_4))
      (:`then_3`
        (bind _returnvalue_5 (`|GetMatProperty` (`self.GetFilePath`) "OPACITY"))
        (`MaterialInstanceDynamic.SetScalarParameterValue` (`self.Mat`) "Op" _returnvalue_5)))))